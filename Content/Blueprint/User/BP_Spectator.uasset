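; Spectator pawn for an agent simulation, with free-fly camera, speed control and save states.
; Holding GameInput switches from cursor-driven UI to game-only input, and scroll-style axis input doubles or halves global time dilation, alongside a pause action.
; Tick accumulates simulation time, which SaveState stores with all BP_AgentBase transforms in indexed BP_Save slots.
; LoadSaveState restores transforms by actor array index; the periodic autosave timer is unconnected.
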(event Custom|Timer
  ;[0.07543 0.08037 0.1146] Simulation Timer
  (Variables|Default|SetTime (+ (Variables|Default|GetTime) (Utilities|Time|GetWorldDeltaSeconds))))

(event Custom|SaveState
  (bind _lastsaveindex (Variables|Default|GetLastSaveIndex))
  (bind _lastsaveindex_2 (Variables|Default|GetLastSaveIndex))
  (bind _saveslot (Utilities|GetSaveSlot _lastsaveindex))
  ;[0.1348 0.2396 0.218] Save & Load Simulation States
  (bind _returnvalue (SaveGame|DoesSaveGameExist _saveslot))
  (if _returnvalue
    (SaveGame|DeleteGameinSlot _saveslot)
    (Utilities|FlowControl|Delay 0.2)
    (CallFunction|SaveState)
    (else
      (bind _outactors (Actor|GetAllActorsOfClass "/Game/Blueprint/Agents/BP_AgentBase.BP_AgentBase_C"))
      (for _array_element _outactors
        (Utilities|Array|Add (Variables|Default|GetAgentLocationsToSave) (Transformation|GetActorTransform _array_element)))
      (bind _returnvalue_2 (SaveGame|CreateSaveGameObject "/Game/Blueprint/User/BP_Save.BP_Save_C"))
      (bind _output_get (Variables|Default|SetSaveGameRef _returnvalue_2))
      (Variables|/Game/Blueprint/User/BP_Save.BP_Save_C|SetAgentLocation _output_get (Variables|Default|GetAgentLocationsToSave))
      (Variables|/Game/Blueprint/User/BP_Save.BP_Save_C|SetTime _output_get (Variables|Default|GetTime))
      (SaveGame|SaveGametoSlot _output_get (Utilities|GetSaveSlot _lastsaveindex_2))
      (Math|Integer|IncrementInt _lastsaveindex_2
        (:%20%20
          (Math|Integer|IncrementInt (Variables|Default|GetMaxSaveIndex)
            (:%20%20
              (Utilities|Array|Clear (Variables|Default|GetAgentLocationsToSave))
              (Development|PrintString "Save Complete!" true true "(R=0.000000,G=1.000000,B=0.260380,A=1.000000)"))))))))

(event Custom|LoadSaveState
  (params (SaveIndex :type Integer))
  (bind _saveslot (Utilities|GetSaveSlot SaveIndex))
  ;[0.1348 0.2396 0.218] Save & Load Simulation States
  (bind _returnvalue (SaveGame|DoesSaveGameExist _saveslot))
  (if _returnvalue
    (bind _returnvalue_2 (SaveGame|LoadGamefromSlot _saveslot))
    (bind _asbp_save (Utilities|Casting|CastToBP_Save _returnvalue_2))
    (bind _outactors (Actor|GetAllActorsOfClass "/Game/Blueprint/Agents/BP_AgentBase.BP_AgentBase_C"))
    (for (_array_element _array_index) _outactors
      (Transformation|SetActorTransform _array_element (Utilities|Array|Get(acopy) (Variables|/Game/Blueprint/User/BP_Save.BP_Save_C|GetAgentLocation _asbp_save) _array_index))
      (Variables|Default|SetTime (Variables|/Game/Blueprint/User/BP_Save.BP_Save_C|GetTime _asbp_save)))
    (Development|PrintString "Load Complete!")))

(event Custom|InitWidget
  (bind _returnvalue (Game|GetPlayerController 0))
  ;[0.05208 0.04042 0.05167] Widget & Controls
  (bind _returnvalue_2 (UserInterface|CreateWidget "/Game/Blueprint/User/UI/UI_Spectator.UI_Spectator_C" _returnvalue))
  (bind _output_get (Variables|Default|SetGameWidget _returnvalue_2))
  (UserInterface|Viewport|AddtoViewport _returnvalue_2 0)
  (Input|SetInputModeGameandUI _returnvalue _output_get "DoNotLock" false false)
  (Variables|/Script/Engine.PlayerController|SetbShowMouseCursor _returnvalue true))

(event EventTick
  (params (DeltaSeconds :type Float%20%28single-precision%29))
  ;[0.07543 0.08037 0.1146] Simulation Timer
  (CallFunction|Timer))

(event EventBeginPlay
  ;[0.3542 0.1731 0.1623] Initialize Timers & Start Simulation
  (CallFunction|InitWidget)
  (bind _returnvalue (UserInterface|CreateWidget "/Game/Blueprint/User/UI/UI_Spectator.UI_Spectator_C"))
  (UserInterface|Viewport|AddtoViewport _returnvalue 0)
  (Game|SetGamePaused false))

(event Input|ActionEvents|InputActionGameInput
  (params (Key :type Key%20Structure :default "None"))
  (bind _returnvalue (Game|GetPlayerController 0))
  ;[0.05208 0.04042 0.05167] Widget & Controls
  (:Pressed
    (Input|SetInputModeGameOnly _returnvalue false)
    (Variables|/Script/Engine.PlayerController|SetbShowMouseCursor _returnvalue false)
    (Variables|Default|SetGameInput true))
  (:Released
    (Input|SetInputModeGameandUI _returnvalue 0 "DoNotLock" false false)
    (Variables|/Script/Engine.PlayerController|SetbShowMouseCursor _returnvalue true)
    (Variables|Default|SetGameInput false)))

(event Input|ActionEvents|InputActionPauseSimulation
  (params (Key :type Key%20Structure :default "None"))
  ;[0.07543 0.08037 0.1146] Time Controls
  (:Pressed
    (Utilities|Time|SetGlobalTimeDilation 0.0)
    (Variables|Default|SetSimulationSpeed 0)))

(event Input|AxisEvents|InputAxisMove_ForwardBackward
  (params (AxisValue :type Float%20%28single-precision%29))
  ;[0.151 0.107 0.07433] Movement
  (Pawn|Input|AddMovementInput (Math|Vector|GetForwardVector (Math|Rotator|MakeRotator 0.0 0.0 (.yaw (Pawn|GetControlRotation :!class /Script/Engine.Pawn)))) AxisValue false))

(event Input|AxisEvents|InputAxisMove_RightLeft
  (params (AxisValue :type Float%20%28single-precision%29))
  (bind _returnvalue (Pawn|GetControlRotation :!class /Script/Engine.Pawn))
  ;[0.151 0.107 0.07433] Movement
  (Pawn|Input|AddMovementInput (Math|Vector|GetRightVector (Math|Rotator|MakeRotator (.roll _returnvalue) 0.0 (.yaw _returnvalue))) AxisValue false))

(event Input|AxisEvents|InputAxisMove_UpDown
  (params (AxisValue :type Float%20%28single-precision%29))
  ;[0.151 0.107 0.07433] Movement
  (Pawn|Input|AddMovementInput (Math|Vector|GetUpVector (Math|Rotator|MakeRotator 0.0 0.0 (.yaw (Pawn|GetControlRotation :!class /Script/Engine.Pawn)))) AxisValue false))

(event Input|AxisEvents|InputAxisMouse_GameSpeed
  (params (AxisValue :type Float%20%28single-precision%29))
  ;[0.07543 0.08037 0.1146] Time Controls
  (if (> AxisValue 0.0)
    (if (== (Variables|Default|GetSimulationSpeed) 0)
      (Utilities|Time|SetGlobalTimeDilation 1.0)
      (Variables|Default|SetSimulationSpeed 1)
      (elif (not (== (Variables|Default|GetSimulationSpeed) 8))
        (Utilities|Time|SetGlobalTimeDilation (Math|Conversions|ToFloat(Integer) (* (Variables|Default|GetSimulationSpeed) 2)))
        (Variables|Default|SetSimulationSpeed (* (Variables|Default|GetSimulationSpeed) 2))))
    (elif (< AxisValue 0.0)
      (Utilities|Time|SetGlobalTimeDilation (Math|Conversions|ToFloat(Integer) (/ (Variables|Default|GetSimulationSpeed) 2)))
      (Variables|Default|SetSimulationSpeed (/ (Variables|Default|GetSimulationSpeed) 2)))))

(event Input|AxisEvents|InputAxisMouse_Up/Down
  (params (AxisValue :type Float%20%28single-precision%29))
  ;[0.151 0.107 0.07433] Movement
  (Pawn|Input|AddControllerPitchInput AxisValue))

(event Input|AxisEvents|InputAxisMouse_Right/Left
  (params (AxisValue :type Float%20%28single-precision%29))
  ;[0.151 0.107 0.07433] Movement
  (Pawn|Input|AddControllerYawInput AxisValue))

(fn ConstructionScript)