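; Deprecated volume that populates a deck with passenger and officer AI agents at random points in its box.
; Looping timers attempt one spawn per tick per type, skipping points blocked by a box trace, until each target count is reached.
; Demographic entries fill in turn by spawn percentage, passing attributes, muster index and deck to each agent.
; Passengers use day or night demographics; officers spawn only in daytime, without stair speeds.
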(event Custom|SpawnPassengerAgent
  (if (< (Variables|Default|GetPassengerAgentsSpawned) (Variables|SpawnProperties|GetPassengerAgents))
    (if (Variables|SpawnProperties|GetbIsDaytime)
      (CallFunction|SpawnPassengerAgentDay)
      (else
        (CallFunction|SpawnPassengerAgentNight)))
    (else
      (Utilities|Time|ClearandInvalidateTimerbyHandle (Variables|Default|GetPassengerAgentSpawnTimer)))))

(event Custom|SpawnPassengerAgentNight
  (bind _currentpassengerdemographicindex (Variables|Attributes|GetCurrentPassengerDemographicIndex))
  (bind _box (Variables|Default|GetBox))
  (bind _nightpassengerdemographics (Variables|Attributes|GetNightPassengerDemographics))
  (bind _agentstatistics (Utilities|Struct|BreakS_NightPassengerAttributesTable _nightpassengerdemographics))
  (bind _output (Utilities|Array|Get(acopy) _agentstatistics _currentpassengerdemographicindex))
  (bind (_spawnpercentage _genderismale_ _agemin _agemax _awarenessmin _awarenessmax _walkspeedonflatmin _walkspeedonflatmax _walkspeedonstairsmin _walkspeedonstairsmax) (Utilities|Struct|BreakS_AgentAttributes _output))
  ;[0.1992 0.1958 0.2552] Spawn Passenger Agents With Night Attributes
  (if (< (Variables|Attributes|GetCurrentDemographicPassengersSpawned) (* _spawnpercentage (/ (Variables|SpawnProperties|GetPassengerAgents) 1e+02)))
    (bind _output_get (Variables|Default|SetPassengerSpawnLocation (Math|Random|RandomPointinBoundingBox (Variables|/Script/Engine.SceneComponent|GetRelativeLocation _box) (Variables|/Script/Engine.BoxComponent|GetBoxExtent _box))))
    (bind _returnvalue (Collision|BoxTraceByChannel _output_get _output_get "21.000000,21.000000,90.000000" "0, 0, 0" "TraceTypeQuery1" false 0 "None" true "(R=1.000000,G=0.000000,B=0.000000,A=1.000000)" "(R=0.000000,G=1.000000,B=0.000000,A=1.000000)" 5e+01))
    (if (not _returnvalue)
      (bind _returnvalue_2 (AI|SpawnAIFromClass "/Game/Blueprint/Agents/BP_AgentBase.BP_AgentBase_C" 0 _output_get "0, 0, 0" true 0))
      (bind _asbp_agent_base (Utilities|Casting|CastToBP_AgentBase _returnvalue_2))
      (Variables|/Game/Blueprint/Agents/BP_AgentBase.BP_AgentBase_C|SetAgentStatistics _asbp_agent_base (Utilities|Struct|MakeS_AgentAttributes _spawnpercentage _genderismale_ _agemin _agemax _awarenessmin _awarenessmax _walkspeedonflatmin _walkspeedonflatmax _walkspeedonstairsmin _walkspeedonstairsmax))
      (Variables|/Game/Blueprint/Agents/BP_AgentBase.BP_AgentBase_C|SetAssignedMusterIndex _asbp_agent_base (Variables|SpawnProperties|GetAsignedAgentMusterIndex))
      (Variables|/Game/Blueprint/Agents/BP_AgentBase.BP_AgentBase_C|SetDeckSpawned _asbp_agent_base (Variables|SpawnProperties|GetCurrentFloor))
      (Math|Integer|IncrementInt (Variables|Attributes|GetCurrentDemographicPassengersSpawned)
        (:%20%20
          (Math|Integer|IncrementInt (Variables|Default|GetPassengerAgentsSpawned)
            (:%20%20
              (Utilities|FlowControl|DoOnce false
                (:Completed
                  (Development|PrintString "Night Demographics"))))))))
    (else
      (Math|Integer|IncrementInt (Variables|Attributes|GetCurrentPassengerDemographicIndex)
        (:%20%20
          (Variables|Attributes|SetCurrentDemographicPassengersSpawned 0))))))

(event Custom|SpawnOfficerAgentDay
  (bind _currentofficerdemographicindex (Variables|Attributes|GetCurrentOfficerDemographicIndex))
  (bind _box (Variables|Default|GetBox))
  (bind _dayofficerdemographics (Variables|Attributes|GetDayOfficerDemographics))
  (bind _agentstatistics (Utilities|Struct|BreakS_DayPassengerAttributesTable _dayofficerdemographics))
  (bind _output (Utilities|Array|Get(acopy) _agentstatistics _currentofficerdemographicindex))
  (bind (_spawnpercentage _genderismale_ _agemin _agemax _awarenessmin _awarenessmax _walkspeedonflatmin _walkspeedonflatmax) (Utilities|Struct|BreakS_AgentAttributes _output))
  ;[0.1904 0.2552 0.1848] Spawn Officer Agents With Day Attributes
  (if (< (Variables|Attributes|GetCurrentDemographicOfficersSpawned) (* _spawnpercentage (/ (Variables|SpawnProperties|GetOfficerAgents) 1e+02)))
    (bind _output_get (Variables|Default|SetOfficerSpawnLocation (Math|Random|RandomPointinBoundingBox (Variables|/Script/Engine.SceneComponent|GetRelativeLocation _box) (Variables|/Script/Engine.BoxComponent|GetBoxExtent _box))))
    (bind _returnvalue (Collision|BoxTraceByChannel _output_get _output_get "21.000000,21.000000,90.000000" "0, 0, 0" "TraceTypeQuery1" false 0 "None" true "(R=1.000000,G=0.000000,B=0.000000,A=1.000000)" "(R=0.000000,G=1.000000,B=0.000000,A=1.000000)" 5e+01))
    (if (not _returnvalue)
      (bind _returnvalue_2 (AI|SpawnAIFromClass "/Game/Blueprint/Agents/BP_OfficerAgent.BP_OfficerAgent_C" 0 _output_get "0, 0, 0" true 0))
      (bind _asbp_agent_base (Utilities|Casting|CastToBP_AgentBase _returnvalue_2))
      (Variables|/Game/Blueprint/Agents/BP_AgentBase.BP_AgentBase_C|SetAgentStatistics _asbp_agent_base (Utilities|Struct|MakeS_AgentAttributes _spawnpercentage _genderismale_ _agemin _agemax _awarenessmin _awarenessmax _walkspeedonflatmin _walkspeedonflatmax))
      (Variables|/Game/Blueprint/Agents/BP_AgentBase.BP_AgentBase_C|SetAssignedMusterIndex _asbp_agent_base (Variables|SpawnProperties|GetAsignedAgentMusterIndex))
      (Variables|/Game/Blueprint/Agents/BP_AgentBase.BP_AgentBase_C|SetDeckSpawned _asbp_agent_base (Variables|SpawnProperties|GetCurrentFloor))
      (Math|Integer|IncrementInt (Variables|Attributes|GetCurrentDemographicOfficersSpawned)
        (:%20%20
          (Math|Integer|IncrementInt (Variables|Default|GetOfficerAgentsSpawned)
            (:%20%20
              (Utilities|FlowControl|DoOnce false
                (:Completed
                  (Development|PrintString "Day Demographics"))))))))
    (else
      (Math|Integer|IncrementInt (Variables|Attributes|GetCurrentOfficerDemographicIndex)
        (:%20%20
          (Variables|Attributes|SetCurrentDemographicOfficersSpawned 0))))))

(event Custom|SpawnOfficerAgent
  (if (< (Variables|Default|GetOfficerAgentsSpawned) (Variables|SpawnProperties|GetOfficerAgents))
    (if (Variables|SpawnProperties|GetbIsDaytime)
      (CallFunction|SpawnOfficerAgentDay))
    (else
      (Utilities|Time|ClearandInvalidateTimerbyHandle (Variables|Default|GetOfficerAgentSpawnTimer)))))

(event Custom|SpawnPassengerAgentDay
  (bind _daypassengerdemographics (Variables|Attributes|GetDayPassengerDemographics))
  (bind _currentpassengerdemographicindex (Variables|Attributes|GetCurrentPassengerDemographicIndex))
  (bind _box (Variables|Default|GetBox))
  (bind _agentstatistics (Utilities|Struct|BreakS_DayPassengerAttributesTable _daypassengerdemographics))
  (bind _output (Utilities|Array|Get(acopy) _agentstatistics _currentpassengerdemographicindex))
  (bind (_spawnpercentage _genderismale_ _agemin _agemax _awarenessmin _awarenessmax _walkspeedonflatmin _walkspeedonflatmax _walkspeedonstairsmin _walkspeedonstairsmax) (Utilities|Struct|BreakS_AgentAttributes _output))
  ;[0.1904 0.2552 0.1848] Spawn Passenger Agents With Day Attributes
  (if (< (Variables|Attributes|GetCurrentDemographicPassengersSpawned) (* _spawnpercentage (/ (Variables|SpawnProperties|GetPassengerAgents) 1e+02)))
    (bind _output_get (Variables|Default|SetPassengerSpawnLocation (Math|Random|RandomPointinBoundingBox (Variables|/Script/Engine.SceneComponent|GetRelativeLocation _box) (Variables|/Script/Engine.BoxComponent|GetBoxExtent _box))))
    (bind _returnvalue (Collision|BoxTraceByChannel _output_get _output_get "21.000000,21.000000,90.000000" "0, 0, 0" "TraceTypeQuery1" false 0 "None" true "(R=1.000000,G=0.000000,B=0.000000,A=1.000000)" "(R=0.000000,G=1.000000,B=0.000000,A=1.000000)" 5e+01))
    (if (not _returnvalue)
      (bind _returnvalue_2 (AI|SpawnAIFromClass "/Game/Blueprint/Agents/BP_AgentBase.BP_AgentBase_C" 0 _output_get "0, 0, 0" true 0))
      (bind _asbp_agent_base (Utilities|Casting|CastToBP_AgentBase _returnvalue_2))
      (Variables|/Game/Blueprint/Agents/BP_AgentBase.BP_AgentBase_C|SetAgentStatistics _asbp_agent_base (Utilities|Struct|MakeS_AgentAttributes _spawnpercentage _genderismale_ _agemin _agemax _awarenessmin _awarenessmax _walkspeedonflatmin _walkspeedonflatmax _walkspeedonstairsmin _walkspeedonstairsmax))
      (Variables|/Game/Blueprint/Agents/BP_AgentBase.BP_AgentBase_C|SetAssignedMusterIndex _asbp_agent_base (Variables|SpawnProperties|GetAsignedAgentMusterIndex))
      (Variables|/Game/Blueprint/Agents/BP_AgentBase.BP_AgentBase_C|SetDeckSpawned _asbp_agent_base (Variables|SpawnProperties|GetCurrentFloor))
      (Math|Integer|IncrementInt (Variables|Attributes|GetCurrentDemographicPassengersSpawned)
        (:%20%20
          (Math|Integer|IncrementInt (Variables|Default|GetPassengerAgentsSpawned)
            (:%20%20
              (Utilities|FlowControl|DoOnce false
                (:Completed
                  (Development|PrintString "Day Demographics"))))))))
    (else
      (Math|Integer|IncrementInt (Variables|Attributes|GetCurrentPassengerDemographicIndex)
        (:%20%20
          (Variables|Attributes|SetCurrentDemographicPassengersSpawned 0))))))

(event EventBeginPlay
  (bind _returnvalue (Utilities|Time|SetTimerbyEvent (delegate Custom|SpawnPassengerAgent) 0.00025 true))
  (Variables|Default|SetPassengerAgentSpawnTimer _returnvalue)
  (bind _returnvalue_2 (Utilities|Time|SetTimerbyEvent (delegate Custom|SpawnOfficerAgent) 0.00025 true))
  (Variables|Default|SetOfficerAgentSpawnTimer _returnvalue_2))

(fn ConstructionScript)