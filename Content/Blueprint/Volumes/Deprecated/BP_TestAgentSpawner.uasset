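; Deprecated test volume that fills its box with passenger agents (BP_AgentBase) for what appears to be a ship muster simulation.
; A fast looping timer tries one random point per tick, spawning only where a box trace is clear, until the passenger target is reached.
; IsFixedWalkSpeed selects day demographics by percentage with a constant walk speed; otherwise agents share one fixed demographic entry.
; Each agent receives its attributes, muster index and deck.
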(event Custom|SpawnPassengerAgent
  (if (< (Variables|Default|GetPassengerAgentsSpawned) (Variables|SpawnProperties|GetPassengerAgents))
    (if (Variables|SpawnProperties|GetbIsFixedWalkSpeed)
      (CallFunction|SpawnFixedWalkSpeed)
      (else
        (CallFunction|SpawnTestMales)))
    (else
      (Utilities|Time|ClearandInvalidateTimerbyHandle (Variables|Default|GetPassengerAgentSpawnTimer)))))

(event Custom|SpawnTestMales
  (bind _daypassengerdemographics (Variables|Attributes|GetDayPassengerDemographics))
  (bind _box (Variables|Default|GetBox))
  (bind _fixedcurrentpassengerdemographics (Variables|Default|GetFixedCurrentPassengerDemographics))
  (bind _agentstatistics (Utilities|Struct|BreakS_DayPassengerAttributesTable _daypassengerdemographics))
  (bind _output (Utilities|Array|Get(acopy) _agentstatistics _fixedcurrentpassengerdemographics))
  (bind (_spawnpercentage _genderismale_ _agemin _agemax _awarenessmin _awarenessmax _walkspeedonflatmin _walkspeedonflatmax) (Utilities|Struct|BreakS_AgentAttributes _output))
  ;[0.1904 0.2552 0.1848] Spawn Passenger Agents With Day Attributes
  (bind _output_get (Variables|Default|SetPassengerSpawnLocation (Math|Random|RandomPointinBoundingBox (Variables|/Script/Engine.SceneComponent|GetRelativeLocation _box) (Variables|/Script/Engine.BoxComponent|GetBoxExtent _box))))
  (bind _returnvalue (Collision|BoxTraceByChannel _output_get _output_get "28.000000,28.000000,90.000000" "0, 0, 0" "TraceTypeQuery1" false 0 "None" true "(R=1.000000,G=0.000000,B=0.000000,A=1.000000)" "(R=0.000000,G=1.000000,B=0.000000,A=1.000000)" 5e+01))
  (if (not _returnvalue)
    (bind _returnvalue_2 (AI|SpawnAIFromClass "/Game/Blueprint/Agents/BP_AgentBase.BP_AgentBase_C" 0 _output_get "0, 0, 0" true 0))
    (bind _asbp_agent_base (Utilities|Casting|CastToBP_AgentBase _returnvalue_2))
    (Variables|/Game/Blueprint/Agents/BP_AgentBase.BP_AgentBase_C|SetAgentStatistics _asbp_agent_base (Utilities|Struct|MakeS_AgentAttributes _spawnpercentage _genderismale_ _agemin _agemax _awarenessmin _awarenessmax _walkspeedonflatmin _walkspeedonflatmax))
    (Variables|/Game/Blueprint/Agents/BP_AgentBase.BP_AgentBase_C|SetAssignedMusterIndex _asbp_agent_base (Variables|SpawnProperties|GetAsignedAgentMusterIndex))
    (Variables|/Game/Blueprint/Agents/BP_AgentBase.BP_AgentBase_C|SetDeckSpawned _asbp_agent_base (Variables|SpawnProperties|GetCurrentFloor))
    (Math|Integer|IncrementInt (Variables|Attributes|GetCurrentDemographicPassengersSpawned)
      (:%20%20
        (Math|Integer|IncrementInt (Variables|Default|GetPassengerAgentsSpawned)
          (:%20%20
            (Utilities|FlowControl|DoOnce false
              (:Completed
                (Development|PrintString "Day Demographics")))))))))

(event Custom|SpawnFixedWalkSpeed
  (bind _currentpassengerdemographicindex (Variables|Attributes|GetCurrentPassengerDemographicIndex))
  (bind _box (Variables|Default|GetBox))
  (bind _daypassengerdemographics (Variables|Attributes|GetDayPassengerDemographics))
  (bind _agentstatistics (Utilities|Struct|BreakS_DayPassengerAttributesTable _daypassengerdemographics))
  (bind _output (Utilities|Array|Get(acopy) _agentstatistics _currentpassengerdemographicindex))
  (bind (_spawnpercentage _genderismale_ _agemin _agemax _awarenessmin _awarenessmax) (Utilities|Struct|BreakS_AgentAttributes _output))
  ;[0.1904 0.2552 0.1848] Spawn Passenger Agents With Day Attributes
  (if (< (Variables|Attributes|GetCurrentDemographicPassengersSpawned) (* _spawnpercentage (/ (Variables|SpawnProperties|GetPassengerAgents) 1e+02)))
    (bind _output_get (Variables|Default|SetPassengerSpawnLocation (Math|Random|RandomPointinBoundingBox (Variables|/Script/Engine.SceneComponent|GetRelativeLocation _box) (Variables|/Script/Engine.BoxComponent|GetBoxExtent _box))))
    (bind _returnvalue (Collision|BoxTraceByChannel _output_get _output_get "28.000000,28.000000,90.000000" "0, 0, 0" "TraceTypeQuery1" false 0 "None" true "(R=1.000000,G=0.000000,B=0.000000,A=1.000000)" "(R=0.000000,G=1.000000,B=0.000000,A=1.000000)" 5e+01))
    (if (not _returnvalue)
      (bind _returnvalue_2 (AI|SpawnAIFromClass "/Game/Blueprint/Agents/BP_AgentBase.BP_AgentBase_C" 0 _output_get "0, 0, 0" true 0))
      (bind _asbp_agent_base (Utilities|Casting|CastToBP_AgentBase _returnvalue_2))
      (Variables|/Game/Blueprint/Agents/BP_AgentBase.BP_AgentBase_C|SetAgentStatistics _asbp_agent_base (Utilities|Struct|MakeS_AgentAttributes _spawnpercentage _genderismale_ _agemin _agemax _awarenessmin _awarenessmax 1e+02 1e+02))
      (Variables|/Game/Blueprint/Agents/BP_AgentBase.BP_AgentBase_C|SetAssignedMusterIndex _asbp_agent_base (Variables|SpawnProperties|GetAsignedAgentMusterIndex))
      (Variables|/Game/Blueprint/Agents/BP_AgentBase.BP_AgentBase_C|SetDeckSpawned _asbp_agent_base (Variables|SpawnProperties|GetCurrentFloor))
      (Math|Integer|IncrementInt (Variables|Attributes|GetCurrentDemographicPassengersSpawned)
        (:%20%20
          (Math|Integer|IncrementInt (Variables|Default|GetPassengerAgentsSpawned)
            (:%20%20
              (Utilities|FlowControl|DoOnce false
                (:Completed
                  (Development|PrintString "Day Demographics"))))))))
    (else
      (Math|Integer|IncrementInt (Variables|Attributes|GetCurrentPassengerDemographicIndex)
        (:%20%20
          (Variables|Attributes|SetCurrentDemographicPassengersSpawned 0))))))

(event EventBeginPlay
  (bind _returnvalue (Utilities|Time|SetTimerbyEvent (delegate Custom|SpawnPassengerAgent) 0.00025 true))
  (Variables|Default|SetPassengerAgentSpawnTimer _returnvalue))

(fn ConstructionScript)