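; BP_MusterStation is a muster station volume that marks agents as mustered in the simulation.
; Agents overlapping MusterBox1 get flagged and added once to the agent array on BP_SimulationStatistics.
; A delayed sweep after BeginPlay applies the same handling to agents already inside the box.
; The assigned-station check on entry is disconnected, and leaving the box does not clear the mustered state.
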(event OnComponentBeginOverlap(MusterBox1)
  (params (OverlappedComponent :type Primitive%20Component%20Object%20Reference) (OtherActor :type Actor%20Object%20Reference) (OtherComp :type Primitive%20Component%20Object%20Reference) (OtherBodyIndex :type Integer) (bFromSweep :type Boolean) (SweepResult :type Hit%20Result%20Structure%20%28by%20ref%29))
  (CallFunction|AgentEnteredMusterStation OtherActor))

(event OnComponentEndOverlap(MusterBox1)
  (params (OverlappedComponent :type Primitive%20Component%20Object%20Reference) (OtherActor :type Actor%20Object%20Reference) (OtherComp :type Primitive%20Component%20Object%20Reference) (OtherBodyIndex :type Integer)))

(event EventBeginPlay
  (bind _outactors (Actor|GetAllActorsOfClass "/Game/Blueprint/Actors/BP_SimulationStatistics.BP_SimulationStatistics_C"))
  (Variables|Default|SetSimulationStatistics (Utilities|Array|Get(acopy) _outactors))
  (Utilities|FlowControl|Delay 5.5)
  (CallFunction|AgentSpawnedinMusterStation (Variables|Default|GetMusterBox1)))

(fn ConstructionScript)

(fn AgentEnteredMusterStation
  (params (Actor :type Actor%20Object%20Reference))
  (bind _simulationstatistics (Variables|Default|GetSimulationStatistics))
  (bind _arrayofagents (Variables|/Game/Blueprint/Actors/BP_SimulationStatistics.BP_SimulationStatistics_C|GetArrayOfAgents _simulationstatistics))
  (bind _asbp_agent_base (Utilities|Casting|CastToBP_AgentBase Actor))
  (Default|AgentMustered _asbp_agent_base true)
  (if (not (Utilities|Array|ContainsItem _arrayofagents _asbp_agent_base))
    (Utilities|Array|Add _arrayofagents _asbp_agent_base)))

(fn AgentLeftMusterStation
  (params (Actor :type Actor%20Object%20Reference))
  (bind _asbp_agent_base (Utilities|Casting|CastToBP_AgentBase Actor))
  (if (== (Variables|/Game/Blueprint/Agents/BP_AgentBase.BP_AgentBase_C|GetAssignedMusterIndex _asbp_agent_base) (Variables|MusterStationProperties|GetMusterStationIndex))
    (Default|AgentMustered _asbp_agent_base false)))

(fn AgentSpawnedinMusterStation
  (params (InMusterBox :type Primitive%20Component%20Object%20Reference))
  (for _array_element (Collision|GetOverlappingActors InMusterBox "/Game/Blueprint/Agents/BP_AgentBase.BP_AgentBase_C" :!class /Script/Engine.PrimitiveComponent)
    (CallFunction|AgentEnteredMusterStation _array_element)))