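; Base agent for a deck-based mustering simulation, representing a person who heads to an assigned muster station.
; After a startup delay it picks a mesh by officer role or gender, then rolls age and walk speeds from AgentStatistics, using fixed speeds in test mode.
; It passes the index-matched muster station to BP_AgentController, starts the simulation, and later relays mustered status.
; Deck assignment also randomly sets a ShouldMaster flag.
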(event EventBeginPlay
  (bind _agentstatistics (Variables|Default|GetAgentStatistics))
  (bind (_spawnpercentage _genderismale_ _agemin _agemax _awarenessmin _awarenessmax _walkspeedonflatmin _walkspeedonflatmax _walkspeedupstairsmin _walkspeedupstairsmax) (Utilities|Struct|BreakS_AgentAttributes _agentstatistics))
  (Utilities|FlowControl|Delay 5.0)
  (CallFunction|SetBaseMesh _genderismale_)
  (Variables|Default|SetAgentAge (Math|Random|RandomIntegerinRange _agemin _agemax))
  (if (Variables|Default|GetbIsTest)
    (CallFunction|SetAttributeSpeed 1e+02 1e+02 1.0)
    (else
      (CallFunction|SetAttributeSpeed (Math|Random|RandomFloatinRange _walkspeedonflatmin _walkspeedonflatmax) (Math|Random|RandomFloatinRange _walkspeedupstairsmin _walkspeedupstairsmax) (Variables|Default|GetAccelerationTime))))
  (CallFunction|SetStatsUI)
  (CallFunction|AgentReacted))

(fn ConstructionScript)

(fn SetBaseMesh
  (params (Male? :type Boolean))
  (bind _mesh (Variables|Character|GetMesh))
  (if (Variables|Default|GetbIsOfficer)
    (Components|SkeletalMesh|SetSkeletalMeshAsset _mesh "/Game/Assets/Agents/SKM_MalePants.SKM_MalePants")
    (elif Male?
      (Components|SkeletalMesh|SetSkeletalMeshAsset _mesh "/Game/Assets/Agents/SKM_MaleShortsBase.SKM_MaleShortsBase")
      (else
        (Components|SkeletalMesh|SetSkeletalMeshAsset _mesh "/Game/Assets/Agents/SKM_FemaleSkirtBase.SKM_FemaleSkirtBase")))))

(fn SetStatsUI
  (Rendering|Components|TextRender|SetText (Variables|Default|GetAgeTextUI) (Utilities|Text|FormatText "Age {Age}" (Variables|Default|GetAgentAge)))
  (Rendering|Components|TextRender|SetText (Variables|Default|GetSpeedTextUI) (Utilities|Text|FormatText "Speed: {Speed}" (Variables|/Script/Engine.CharacterMovementComponent|GetMaxWalkSpeed (Variables|Character|GetCharacterMovement)))))

(fn SetCurrentDeck
  (params (InDeck :type Integer) (InFloorSize :type Vector) (InFloorLocation :type Vector))
  (Variables|Default|SetCurrentDeck InDeck)
  (Variables|Default|SetCurrentDeckSize InFloorSize)
  (Variables|Default|SetCurrentDeckLocation InFloorLocation)
  (Variables|Default|SetbShouldMaster (!= (Math|Random|RandomIntegerinRange 1 10) 10)))

(fn AgentReacted
  (bind _asbp_agent_controller (Utilities|Casting|CastToBP_AgentController (AI|GetAIController self)))
  (bind _output_get (Variables|Default|SetAgentController _asbp_agent_controller))
  (bind _outactors (Actor|GetAllActorsOfClass "/Game/Blueprint/Volumes/MusterStation/BP_MusterStation.BP_MusterStation_C"))
  (for _array_element _outactors
    (if (== (Variables|/Game/Blueprint/Volumes/MusterStation/BP_MusterStation.BP_MusterStation_C|GetMusterStationIndex _array_element) (Variables|Default|GetAssignedMusterIndex))
      (Default|SetMusterStation _output_get _array_element)))
  (Default|StartSimulation _output_get))

(fn AgentMustered
  (params (Mustered? :type Boolean))
  (bind _asbp_agent_controller (Utilities|Casting|CastToBP_AgentController (AI|GetAIController self)))
  (Default|AgentMustered _asbp_agent_controller Mustered?)
  (bind _output_get (Variables|Default|SetbHasMustered Mustered?))
  (if _output_get
    (Rendering|Components|Sprite|SetSprite (Variables|Default|GetBillboard) "/Game/Assets/Materials/Textures/Billboards/T_Checkmark.T_Checkmark")
    (else
      (CallFunction|SetBaseMesh (.GenderIsMale? (Utilities|Struct|BreakS_AgentAttributes (Variables|Default|GetAgentStatistics)))))))

(fn SetAttributeSpeed
  (params (InWalkSpeedOnFlat :type Float%20%28single-precision%29) (InWalkSpeedOnStairs :type Float%20%28single-precision%29) (InAccelerationTime :type Float%20%28double-precision%29))
  (bind _charactermovement (Variables|Character|GetCharacterMovement))
  (bind _output_get (Variables|/Script/Engine.CharacterMovementComponent|SetMaxWalkSpeed _charactermovement InWalkSpeedOnFlat))
  (bind _output_get_2 (Variables|Default|SetWalkSpeedOnFlat _output_get))
  (Variables|/Script/Engine.CharacterMovementComponent|SetMaxAcceleration _charactermovement (/ _output_get_2 InAccelerationTime))
  (Variables|Default|SetWalkSpeedOnStairs InWalkSpeedOnStairs))