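; BP_AgentController is the AI controller for simulation agents that react and head to muster stations.
; It runs the BT_AgentBase behavior tree on BeginPlay and enables move block detection at construction.
; Its events feed that tree through Blackboard keys for reaction, mustered state and target muster station.
; A further event swaps the default navigation filter class, allowing pathfinding rules to be set per agent.
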(event Custom|SetMusterStation
  (params (MusterStation :type BP%20Muster%20Station%20Object%20Reference))
  (AI|Components|Blackboard|SetValueasObject (Variables|Default|GetBlackboard) (Utilities|Name|MakeLiteralName "TargetMusterStation") MusterStation))

(event Custom|StartSimulation
  (AI|Components|Blackboard|SetValueasBool (Variables|Default|GetBlackboard) (Utilities|Name|MakeLiteralName "bAgentReacted") true))

(event Custom|SetNavFilter
  (params (Filter :type Navigation%20Query%20Filter%20Class%20Reference))
  (Variables|Default|SetDefaultNavigationFilterClass Filter))

(event Custom|AgentMustered
  (params (Mustered? :type Boolean))
  (AI|Components|Blackboard|SetValueasBool (Variables|Default|GetBlackboard) (Utilities|Name|MakeLiteralName "bAgentMustered") Mustered?))

(event EventBeginPlay
  (AI|RunBehaviorTree "/Game/Blueprint/Agents/AI/BT_AgentBase.BT_AgentBase"))

(fn ConstructionScript
  (Class|AIController|SetMoveBlockDetection true))