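; Daytime attribute handler that assigns demographic statistics (gender and ranges for age, awareness and walk speeds) to passenger and officer agents already in the level.
; On BeginPlay it gathers both agent arrays, then after short delays starts very fast looping timers, the officer one only if officers exist.
; Each timer call gives a random remaining agent the current demographic, or advances once its scaled SpawnPercentage quota is met, stopping when the array empties.
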(event Custom|SetOfficerStatistics
  (bind _dayofficerdemographics (Variables|Officers|GetDayOfficerDemographics))
  (bind _currentofficerdemographicindex (Variables|Officers|GetCurrentOfficerDemographicIndex))
  (bind _officerarray (Variables|Officers|GetOfficerArray))
  (bind _agentstatistics (Utilities|Struct|BreakS_DayOfficersAttributesTable _dayofficerdemographics))
  (bind _output (Utilities|Array|Get(acopy) _agentstatistics _currentofficerdemographicindex))
  (bind (_spawnpercentage _genderismale_ _agemin _agemax _awarenessmin _awarenessmax _walkspeedonflatmin _walkspeedonflatmax _walkspeedonstairsmin _walkspeedonstairsmax) (Utilities|Struct|BreakS_AgentAttributes _output))
  (if (< (Variables|Officers|GetCurrentDemographicOfficersSpawned) (* _spawnpercentage 0.85))
    (bind _output_get (Variables|Officers|SetCurrentOfficer (.OutItem (Utilities|Array|Random (Variables|Officers|GetOfficerArray)))))
    (Variables|/Game/Blueprint/Agents/BP_AgentBase.BP_AgentBase_C|SetAgentStatistics _output_get (Utilities|Struct|MakeS_AgentAttributes _spawnpercentage _genderismale_ _agemin _agemax _awarenessmin _awarenessmax _walkspeedonflatmin _walkspeedonflatmax _walkspeedonstairsmin _walkspeedonstairsmax))
    (Math|Integer|IncrementInt (Variables|Officers|GetCurrentDemographicOfficersSpawned)
      (:%20%20
        (Utilities|Array|RemoveItem _officerarray _output_get)
        (if (Utilities|Array|IsEmpty _officerarray)
          (Utilities|Time|ClearandInvalidateTimerbyHandle (Variables|Officers|GetOfficerAttributeSetTimer)))))
    (else
      (Math|Integer|IncrementInt (Variables|Officers|GetCurrentOfficerDemographicIndex)
        (:%20%20
          (Variables|Officers|SetCurrentDemographicOfficersSpawned 0))))))

(event Custom|SetPassengerStatistics
  (bind _currentpassengerdemographicindex (Variables|Passengers|GetCurrentPassengerDemographicIndex))
  (bind _passengerarray (Variables|Passengers|GetPassengerArray))
  (bind _daypassengerdemographics (Variables|Passengers|GetDayPassengerDemographics))
  (bind _agentstatistics (Utilities|Struct|BreakS_DayPassengerAttributesTable _daypassengerdemographics))
  (bind _output (Utilities|Array|Get(acopy) _agentstatistics _currentpassengerdemographicindex))
  (bind (_spawnpercentage _genderismale_ _agemin _agemax _awarenessmin _awarenessmax _walkspeedonflatmin _walkspeedonflatmax _walkspeedonstairsmin _walkspeedonstairsmax) (Utilities|Struct|BreakS_AgentAttributes _output))
  (if (< (Variables|Passengers|GetCurrentDemographicPassengersSpawned) (* _spawnpercentage 24.0))
    (bind _output_get (Variables|Passengers|SetCurrentAgent (.OutItem (Utilities|Array|Random (Variables|Passengers|GetPassengerArray)))))
    (Variables|/Game/Blueprint/Agents/BP_AgentBase.BP_AgentBase_C|SetAgentStatistics _output_get (Utilities|Struct|MakeS_AgentAttributes _spawnpercentage _genderismale_ _agemin _agemax _awarenessmin _awarenessmax _walkspeedonflatmin _walkspeedonflatmax _walkspeedonstairsmin _walkspeedonstairsmax))
    (Math|Integer|IncrementInt (Variables|Passengers|GetCurrentDemographicPassengersSpawned)
      (:%20%20
        (Utilities|Array|RemoveItem _passengerarray _output_get)
        (if (Utilities|Array|IsEmpty _passengerarray)
          (Utilities|Time|ClearandInvalidateTimerbyHandle (Variables|Passengers|GetPassengerAttributeSetTimer)))))
    (else
      (Math|Integer|IncrementInt (Variables|Passengers|GetCurrentPassengerDemographicIndex)
        (:%20%20
          (Variables|Passengers|SetCurrentDemographicPassengersSpawned 0))))))

(event EventBeginPlay
  (bind _outactors (Actor|GetAllActorsOfClass "/Game/Blueprint/Agents/BP_AgentBase.BP_AgentBase_C"))
  (Variables|Passengers|SetPassengerArray _outactors)
  (bind _outactors_2 (Actor|GetAllActorsOfClass "/Game/Blueprint/Agents/BP_OfficerAgent.BP_OfficerAgent_C"))
  (Variables|Officers|SetOfficerArray _outactors_2)
  (Utilities|FlowControl|Delay 0.5)
  (bind _returnvalue (Utilities|Time|SetTimerbyEvent (delegate Custom|SetPassengerStatistics) 0.00025 true))
  (Variables|Passengers|SetPassengerAttributeSetTimer _returnvalue)
  (Utilities|FlowControl|Delay 0.7)
  (if (> (Utilities|Array|Length (Variables|Officers|GetOfficerArray)) 0)
    (bind _returnvalue_2 (Utilities|Time|SetTimerbyEvent (delegate Custom|SetOfficerStatistics) 0.00025 true))
    (Variables|Officers|SetOfficerAttributeSetTimer _returnvalue_2)))

(fn ConstructionScript)