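; BP_TestAttributeHandler is a test actor that assigns demographic statistics to every BP_AgentBase agent in the level.
; On BeginPlay it gathers the agents and, after a short delay, starts a very fast looping timer.
; Each tick picks a random remaining agent, disables its movement and copies in the DayPassengerDemographics entry at CurrentPassengerDemographicIndex, which this graph never changes.
; Processed agents leave the array, and the timer clears once it is empty.
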(event Custom|SetPassengerStatistics
  (bind _currentpassengerdemographicindex (Variables|Passengers|GetCurrentPassengerDemographicIndex))
  (bind _passengerarray (Variables|Passengers|GetPassengerArray))
  (bind _daypassengerdemographics (Variables|Passengers|GetDayPassengerDemographics))
  (bind _agentstatistics (Utilities|Struct|BreakS_DayPassengerAttributesTable _daypassengerdemographics))
  (bind _output (Utilities|Array|Get(acopy) _agentstatistics _currentpassengerdemographicindex))
  (bind (_spawnpercentage _genderismale_ _agemin _agemax _awarenessmin _awarenessmax _walkspeedonflatmin _walkspeedonflatmax _walkspeedonstairsmin _walkspeedonstairsmax) (Utilities|Struct|BreakS_AgentAttributes _output))
  (bind _output_get (Variables|Passengers|SetCurrentAgent (.OutItem (Utilities|Array|Random (Variables|Passengers|GetPassengerArray)))))
  (Pawn|Components|CharacterMovement|DisableMovement (Variables|/Script/Engine.Character|GetCharacterMovement _output_get))
  (Variables|/Game/Blueprint/Agents/BP_AgentBase.BP_AgentBase_C|SetAgentStatistics _output_get (Utilities|Struct|MakeS_AgentAttributes _spawnpercentage _genderismale_ _agemin _agemax _awarenessmin _awarenessmax _walkspeedonflatmin _walkspeedonflatmax _walkspeedonstairsmin _walkspeedonstairsmax))
  (Utilities|Array|RemoveItem _passengerarray _output_get)
  (if (Utilities|Array|IsEmpty _passengerarray)
    (Utilities|Time|ClearandInvalidateTimerbyHandle (Variables|Passengers|GetPassengerAttributeSetTimer))))

(event EventBeginPlay
  (bind _outactors (Actor|GetAllActorsOfClass "/Game/Blueprint/Agents/BP_AgentBase.BP_AgentBase_C"))
  (Variables|Passengers|SetPassengerArray _outactors)
  (Utilities|FlowControl|Delay 0.5)
  (bind _returnvalue (Utilities|Time|SetTimerbyEvent (delegate Custom|SetPassengerStatistics) 0.00025 true))
  (Variables|Passengers|SetPassengerAttributeSetTimer _returnvalue))

(fn ConstructionScript)