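; BP_SimulationStatistics is an actor that tracks how many simulation agents have mustered.
; On BeginPlay it records the total BP_AgentBase count and starts a looping timer.
; Each tick of that timer re-gathers all agents, recounts those with HasMustered set, and writes the running count to the first SimulationManager's MusteredAgents.
; That write happens only when a mustered agent is found, so a zero count is never pushed.
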(event Custom|Find%20Mustered%20Agents
  (Variables|Default|SetTotalMusteredAgents 0)
  (bind _outactors (Actor|GetAllActorsOfClass "/Game/Blueprint/Agents/BP_AgentBase.BP_AgentBase_C"))
  (for _array_element _outactors
    (if (Variables|/Script/ShipEvacuationSim.AiCharacter|GetbHasMustered _array_element)
      (Math|Integer|IncrementInt (Variables|Default|GetTotalMusteredAgents)
        (:%20%20
          (bind _outactors_2 (Actor|GetAllActorsOfClass "/Script/ShipEvacuationSim.SimulationManager"))
          (Variables|/Script/ShipEvacuationSim.SimulationManager|SetMusteredAgents (Utilities|Array|Get(acopy) _outactors_2) (Variables|Default|GetTotalMusteredAgents)))))))

(event EventBeginPlay
  (bind _outactors (Actor|GetAllActorsOfClass "/Game/Blueprint/Agents/BP_AgentBase.BP_AgentBase_C"))
  (bind _output_get (Variables|Default|SetArrayOfAgents _outactors))
  (Variables|Default|SetTotalSimulationAgents (Utilities|Array|Length _output_get))
  (Utilities|Time|SetTimerbyEvent (delegate Custom|Find%20Mustered%20Agents) 2.0 true))

(fn ConstructionScript)