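; Niagara fire effect actor that spawns fire from a posed skeletal mesh, with optional point light.
; The construction script applies the configured mesh, Niagara system, mesh scale and light settings.
; BeginPlay plays an animation, pauses it after a set delay, then starts a timeline.
; Timeline updates feed Niagara the mesh, emitter toggles, angle limit, scale and a randomly jittered fire direction, optionally oscillating, and activate it.
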(event EventBeginPlay
  (bind _niagara (Variables|Default|GetNiagara))
  (bind _skeletalmesh (Variables|Default|GetSkeletalMesh))
  (bind _ani_seq (Variables|FireSettings|GetAni_Seq))
  (bind _random_start_angle_max (Variables|FireAngle|GetRandom_Start_angle_max))
  (bind _random_start_angle_min (Variables|FireAngle|GetRandom_Start_angle_min))
  (bind _returnvalue (Math|Random|RandomFloatinRange _random_start_angle_min _random_start_angle_max))
  (bind _returnvalue_2 (Math|Vector|MakeVector _returnvalue _returnvalue 0.0))
  (Components|Activation|SetActive (Variables|Default|GetNiagara) false false)
  (Rendering|SetVisibility (Variables|Default|GetPointLight) (Variables|FireLight|GetLight) false)
  (Components|Animation|SetAnimation _skeletalmesh _ani_seq)
  (Components|Activation|SetActive _skeletalmesh true true)
  (Components|Animation|PlayAnimation _skeletalmesh _ani_seq false)
  (Utilities|FlowControl|Delay (Variables|FireSettings|Getanimation_stop_position))
  (Variables|/Script/Engine.SkeletalMeshComponent|SetbPauseAnims (Variables|Default|GetSkeletalMesh) true)
  (Components|Timeline|SetPlayRate (Variables|Default|GetTimeline_1) (Variables|FireOscillator|GetOscil_Speed))
  (bind _dir_vector (Timeline|Timeline_1 Play)
    (:Update
      (CallFunction|SetVariableVec3 (Variables|Default|GetNiagara) "User.Direction" (select (Variables|FireOscillator|Getoscillate) (Math|Vector|Normalize (+ _dir_vector _returnvalue_2)) (Math|Vector|Normalize (+ (Variables|FireTransform|GetFire_Direction) _returnvalue_2))))
      (CallFunction|OverrideSystemUserVariableSkeletalMeshComponent (Variables|Default|GetNiagara) "User.SpawnSMesh" (Variables|Default|GetSkeletalMesh))
      (CallFunction|SetVariableFloat _niagara "User.Smoke" (Math|Conversions|ToFloat(Boolean) (Variables|FireSettings|GetSmoke_Emitter_Enable)))
      (CallFunction|SetVariableFloat _niagara "User.Distortion" (Math|Conversions|ToFloat(Boolean) (Variables|FireSettings|GetDistortion_Emittter_Enable)))
      (CallFunction|SetVariableFloat _niagara "User.FireAngleLimit" (Variables|FireSettings|GetFireAngleLimit))
      (Transformation|SetRelativeScale3D _niagara (Variables|FireTransform|GetFireScale))
      (Components|Activation|SetActive (Variables|Default|GetNiagara) true false))))

(fn ConstructionScript
  (bind _skeletalmesh (Variables|Default|GetSkeletalMesh))
  (bind _pointlight (Variables|Default|GetPointLight))
  (Components|SkinnedMesh|SetSkinnedAssetandUpdate _skeletalmesh (Variables|FireSettings|Getskel_mesh) true)
  (Transformation|SetWorldScale3D _skeletalmesh (Variables|FireSettings|Getskelmesh_scale))
  (Rendering|Components|Light|SetIntensity _pointlight (Variables|FireLight|GetLight_Intensity))
  (Rendering|Lighting|SetAttenuationRadius _pointlight (Variables|FireLight|GetLightRadius))
  (CallFunction|SetAsset (Variables|Default|GetNiagara) (.NiagaraAsset (Variables|FireSettings|GetNiagaraAsset)) true)
  (CallFunction|OverrideSystemUserVariableSkeletalMeshComponent (Variables|Default|GetNiagara) "User.SpawnSMesh" (Variables|Default|GetSkeletalMesh)))