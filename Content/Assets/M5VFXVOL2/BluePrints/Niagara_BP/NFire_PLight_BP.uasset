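; Niagara fire effect actor with an optional point light and tunable scale, smoke, distortion and angle limit.
; The construction script assigns the Niagara asset and configures the light, scaling its radius by the fire's X scale.
; On BeginPlay it pushes user parameters and activates the effect, using a fixed direction or a timeline-driven oscillating one.
; Random X/Y jitter is added to the direction, re-rolled on every timeline update when oscillating.
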(event EventBeginPlay
  (bind _niagara (Variables|Default|GetNiagara))
  (bind _random_start_angle_max (Variables|FireAngle|GetRandom_Start_angle_max))
  (bind _random_start_angle_min (Variables|FireAngle|GetRandom_Start_angle_min))
  (bind _returnvalue (Math|Random|RandomFloatinRange _random_start_angle_min _random_start_angle_max))
  (bind _returnvalue_2 (Math|Vector|MakeVector _returnvalue _returnvalue 0.0))
  (Components|Timeline|SetPlayRate (Variables|Default|GetTimeline_0) (Variables|FireOscillator|GetOscil_Speed))
  (if (Variables|FireOscillator|Getoscillate)
    (bind _dir_vector (Timeline|Timeline_0 Play)
      (:Update
        _)))
  (CallFunction|SetVariableVec3 _niagara "User.Direction" (select (Variables|FireOscillator|Getoscillate) (Math|Vector|Normalize (+ _dir_vector _returnvalue_2)) (Math|Vector|Normalize (+ (Variables|FireTransform|GetDirection) _returnvalue_2))))
  (CallFunction|SetVariableFloat _niagara "User.Smoke" (Math|Conversions|ToFloat(Boolean) (Variables|FireSettings|GetSmoke_Emitter_Enable)))
  (CallFunction|SetVariableFloat _niagara "User.Distortion" (Math|Conversions|ToFloat(Boolean) (Variables|FireSettings|GetDistortion_Emittter_Enable)))
  (CallFunction|SetVariableFloat _niagara "User.FireAngleLimit" (Variables|FireTransform|GetFireAngleLimit))
  (Transformation|SetRelativeScale3D _niagara (Variables|FireTransform|GetFireScale))
  (Components|Activation|SetActive _niagara true false))

(fn ConstructionScript
  (bind _pointlight (Variables|Default|GetPointLight))
  ;[1 1 1] Light
  (Rendering|SetVisibility _pointlight (Variables|FireLight|GetLight) false)
  (Rendering|Components|Light|SetIntensity _pointlight (Variables|FireLight|GetLight_Intensity))
  (Rendering|Lighting|SetAttenuationRadius _pointlight (* (Variables|FireLight|GetLightRadius) (.x (Variables|FireTransform|GetFireScale))))
  (CallFunction|SetAsset (Variables|Default|GetNiagara) (.NiagaraAsset (Variables|FireSettings|GetNiagaraAsset)) true))