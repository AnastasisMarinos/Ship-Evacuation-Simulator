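; Configurable Niagara fire beam effect actor with an optional oscillating, shaking end point.
; Construction script applies the mesh, Niagara asset and scales, places start and end arrows from offsets, and feeds endpoints, direction and width to Niagara.
; BeginPlay sets smoke and distortion toggles, then nested timelines move the end arrow by optional oscillation plus random-speed shake noise.
; Updates push endpoints and a direction normalized from the end position alone.
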(event EventBeginPlay
  (bind _niagara (Variables|Default|GetNiagara))
  (bind _niagara_2 (Variables|Default|GetNiagara))
  (bind _niagara_3 (Variables|Default|GetNiagara))
  (Variables|FireTransform|Setorigin_top_position (Variables|/Script/Engine.SceneComponent|GetRelativeLocation (Variables|Default|GetArrow1)))
  (CallFunction|SetVariableFloat _niagara_3 "User.Smoke" (Math|Conversions|ToFloat(Boolean) (Variables|FireSettings|GetSmoke_Emitter_Enable)))
  (CallFunction|SetVariableFloat _niagara_3 "User.Distortion" (Math|Conversions|ToFloat(Boolean) (Variables|FireSettings|GetDistortion_Emittter_Enable)))
  (Components|Timeline|SetPlayRate (Variables|Default|GetTimeline_0) (Variables|FireOscillator|GetOscil_Speed))
  (bind _dir_vector (Timeline|Timeline_0 Play)
    (:Update
      (CallFunction|SetVariableVec3 _niagara "User.Beam Start" (Variables|/Script/Engine.SceneComponent|GetRelativeLocation (Variables|Default|GetArrow)))
      (CallFunction|SetVariableVec3 _niagara "User.Beam End" (Variables|/Script/Engine.SceneComponent|GetRelativeLocation (Variables|Default|GetArrow1)))
      (Components|Timeline|SetPlayRate (Variables|Default|GetTimeline_1) (Math|Random|RandomFloatinRange (Variables|FireShake|Getshake_speed_min) (Variables|FireShake|Getshake_speed_max)))
      (bind _random_mul (Timeline|Timeline_1 Play)
        (:Update
          (Transformation|SetRelativeLocation (Variables|Default|GetArrow1) (select (Variables|FireOscillator|Getoscillate) (+ (Variables|FireTransform|Getorigin_top_position) (+ (* _dir_vector (Variables|FireOscillator|Getoscil_scale)) (* _random_mul (Variables|FireShake|Getshake_noise_scale)))) (+ (Variables|FireTransform|Getorigin_top_position) (* _random_mul (Variables|FireShake|Getshake_noise_scale)))) false false)
          (CallFunction|SetVariableVec3 _niagara_2 "User.Direction" (Math|Vector|Normalize (select (Variables|FireOscillator|Getoscillate) (+ (Variables|FireTransform|Getorigin_top_position) (+ (* _dir_vector (Variables|FireOscillator|Getoscil_scale)) (* _random_mul (Variables|FireShake|Getshake_noise_scale)))) (+ (Variables|FireTransform|Getorigin_top_position) (* _random_mul (Variables|FireShake|Getshake_noise_scale))))))
          (Components|Activation|SetActive _niagara_2 true false))))))

(fn ConstructionScript
  (bind _staticmeshcomponent (Variables|Debug|GetStaticMeshComponent))
  (bind _niagara (Variables|Default|GetNiagara))
  (Components|StaticMesh|SetStaticMesh _staticmeshcomponent (Variables|FireSettings|GetStaticmesh))
  (Transformation|SetRelativeScale3D _staticmeshcomponent (Variables|FireTransform|GetScale))
  (Transformation|SetRelativeLocation (Variables|Default|GetSphere) (Variables|FireTransform|GetBase_position) false false)
  (CallFunction|SetAsset _niagara (.NiagaraAsset (Variables|FireSettings|GetNiagaraAsset)) true)
  (Transformation|SetRelativeLocation (Variables|Default|GetArrow) (Variables|FireTransform|GetStart_offset) false false)
  (Transformation|SetRelativeLocation (Variables|Default|GetArrow1) (Variables|FireTransform|GetEnd_offset) false false)
  (Transformation|SetRelativeScale3D _niagara (Variables|FireTransform|GetParticle_Scale))
  (CallFunction|SetVariableVec3 _niagara "User.Beam Start" (Variables|/Script/Engine.SceneComponent|GetRelativeLocation (Variables|Default|GetArrow)))
  (CallFunction|SetVariableVec3 _niagara "User.Beam End" (Variables|/Script/Engine.SceneComponent|GetRelativeLocation (Variables|Default|GetArrow1)))
  (CallFunction|SetVariableVec3 (Variables|Default|GetNiagara) "User.Direction" (Math|Vector|Normalize (Math|Vector|GetUnitDirection(Vector) (Variables|FireTransform|GetStart_offset) (Variables|FireTransform|GetEnd_offset))))
  (CallFunction|SetVariableFloat _niagara "User.Beam Width" (Variables|FireSettings|Getbeam_width)))