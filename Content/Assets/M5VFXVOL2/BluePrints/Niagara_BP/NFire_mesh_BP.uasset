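; Actor Blueprint that pairs a configurable static mesh with a Niagara fire effect.
; The construction script applies the chosen mesh and scale.
; On BeginPlay it assigns the Niagara asset, offsets and scales it, and pushes smoke, distortion and fire-angle settings into Niagara user parameters.
; The angle limit is normalised, with 1 meaning 180 degrees.
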(event EventBeginPlay
  (bind _niagara (Variables|Default|GetNiagara))
  (bind _niagara_2 (Variables|Default|GetNiagara))
  (CallFunction|SetAsset _niagara_2 (.NiagaraAsset (Variables|FireSettings|GetNiagaraAsset)) true)
  (Transformation|SetRelativeLocation _niagara_2 (Variables|FireSettings|GetParticle_offset) false false)
  (Transformation|SetRelativeScale3D _niagara_2 (Variables|FireSettings|GetParticle_Scale))
  (CallFunction|SetVariableFloat _niagara "User.Smoke" (Math|Conversions|ToFloat(Boolean) (Variables|FireSettings|GetSmoke_Emitter_Enable)))
  (CallFunction|SetVariableFloat _niagara "User.Distortion" (Math|Conversions|ToFloat(Boolean) (Variables|FireSettings|GetDistortion_Emittter_Enable)))
  (CallFunction|SetVariableFloat _niagara "User.FireAngleLimit" (Variables|FireSettings|GetFireAngleLimit)))

(fn ConstructionScript
  (bind _staticmeshcomponent (Variables|Debug|GetStaticMeshComponent))
  (Components|StaticMesh|SetStaticMesh _staticmeshcomponent (Variables|FireSettings|GetStaticmesh))
  (Transformation|SetRelativeScale3D _staticmeshcomponent (Variables|FireSettings|GetScale)))